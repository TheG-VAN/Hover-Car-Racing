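; Finish line checkpoint for the hover car race, which completes a car's lap.
; Initialise links NextCP to the Checkpoint_BP actor numbered 1.
; On overlap, a HoverCar expecting this checkpoint number has its next checkpoint reset to 1, triggers a new lap and plays a confirm sound.
; It also moves that car's respawn transform to the finish actor, raised by the car's hover distance.
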(event Collision|EventActorBeginOverlap
  (params (OtherActor :type Actor%20Object%20Reference))
  (bind _ashover_car (Utilities|Casting|CastToHoverCar OtherActor))
  (if (== (Variables|/Game/HoverCar/HoverCar.HoverCar_C|GetNextCheckpoint _ashover_car) (Variables|Default|GetCheckpointNum))
    (Variables|/Game/HoverCar/HoverCar.HoverCar_C|SetNextCheckpoint _ashover_car 1)
    (Audio|PlaySoundatLocation "/Engine/VREditor/Sounds/VR_confirm_Cue.VR_confirm_Cue" (Transformation|GetActorLocation) "0, 0, 0" 1.0 1.0 0.0 0 0 0 0)
    (Default|NewLap _ashover_car)
    ;[1 1 1] Set respawn location
    (Variables|/Game/HoverCar/HoverCar.HoverCar_C|SetRespawnTransform _ashover_car (Math|Transform|MakeTransform (+ (Transformation|GetActorLocation) (Math|Vector|MakeVector 0.0 0.0 (Variables|/Game/HoverCar/HoverCar.HoverCar_C|GetHoverDistance _ashover_car))) (Transformation|GetActorRotation) (Transformation|GetActorScale3D _ashover_car)))))

(event EventTick
  (params (DeltaSeconds :type Float%20%28single-precision%29)))

(event EventInitialise
  (bind _outactors (Actor|GetAllActorsOfClass "/Game/Track/Checkpoint_BP.Checkpoint_BP_C"))
  (bind _array_element (Utilities|Array|ForEachLoopwithBreak _outactors)
    (:LoopBody
      (if (== (Variables|/Game/Track/Checkpoint_BP.Checkpoint_BP_C|GetCheckpointNum _array_element) 1)
        (Variables|Default|SetNextCP _array_element)))))

(fn ConstructionScript
  (|CallParentFunction))